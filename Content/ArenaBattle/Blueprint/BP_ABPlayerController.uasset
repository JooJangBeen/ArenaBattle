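; Player controller for the ArenaBattle game that builds the HUD and relays game state to the UI.
; On BeginPlay it creates the HUD, caches its score widget and seeds it with the game mode's clear score.
; Score and retry-count events update that widget, while game over and game clear share one path showing a result widget with the success flag.
; A clear also spawns a congratulation actor at the controlled pawn's location.
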(event EventOnGameRetryCount
  (params (NewRetryCount :type Integer))
  (Default|SetRetryCount (Variables|Default|GetScoreWidget) NewRetryCount))

(event EventOnScoreChanged
  (params (NewScore :type Integer))
  (Default|SetScore (Variables|Default|GetScoreWidget) NewScore))

(event EventOnGameOver
  (Variables|Default|SetIsSuccess false)
  (bind _returnvalue (UserInterface|CreateWidget "/Game/ArenaBattle/UI/WBP_GameResult.WBP_GameResult_C"))
  (UserInterface|Viewport|AddtoViewport _returnvalue 0)
  (Default|SetResult _returnvalue (Variables|Default|GetIsSuccess)))

(event EventOnGameClear
  (Variables|Default|SetIsSuccess true)
  (Utilities|FlowControl|Sequence
    (:then_0
      (bind _returnvalue (UserInterface|CreateWidget "/Game/ArenaBattle/UI/WBP_GameResult.WBP_GameResult_C"))
      (UserInterface|Viewport|AddtoViewport _returnvalue 0)
      (Default|SetResult _returnvalue (Variables|Default|GetIsSuccess)))
    (:then_1
      (Game|SpawnActorfromClass "/Game/ArenaBattle/Blueprint/BP_Congratulation.BP_Congratulation_C" (Math|Transform|MakeTransform (Transformation|GetActorLocation (Pawn|GetControlledPawn)) "0, 0, 0" "1.000000,1.000000,1.000000") "Undefined" "MultiplyWithRoot" 0 0))))

(event EventBeginPlay
  (bind _returnvalue (UserInterface|CreateWidget "/Game/ArenaBattle/UI/WBP_ABHUD.WBP_ABHUD_C"))
  (UserInterface|Viewport|AddtoViewport _returnvalue 0)
  (Variables|Default|SetScoreWidget (Variables|/Game/ArenaBattle/UI/WBP_ABHUD.WBP_ABHUD_C|GetWBP_PlayerScore _returnvalue))
  (bind _asbp_abgame_mode (Utilities|Casting|CastToBP_ABGameMode (Game|GetGameMode)))
  (Default|SetClearScore (Variables|Default|GetScoreWidget) (Variables|/Script/ArenaBattleDemo.ABGameMode|GetClearScore _asbp_abgame_mode)))

(fn ConstructionScript)